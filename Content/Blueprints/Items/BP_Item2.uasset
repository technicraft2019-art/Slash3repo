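; BP_Item2 is an item actor that moves horizontally every Tick by adding a world offset from TransformedSin on X and TransformedCos on Y.
; Unconnected example graphs show clamping Amplitude, a variable noted as created in C++, and bobbing the actor vertically with a sine wave; neither runs.
; BeginPlay, overlap and the construction script are empty.
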(event `self.ReceiveTick`
  (params (DeltaSeconds :type "Float (single-precision)"))
  (`self.K2_AddActorWorldOffset` (`KismetMathLibrary.MakeVector` (`self.TransformedSin`) (`self.TransformedCos`))))

(fn `UserConstructionScript`)