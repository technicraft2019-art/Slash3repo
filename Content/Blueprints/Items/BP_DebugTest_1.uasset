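; Debug test actor that draws a moving sphere with a sweeping line.
; Each Tick calls LineSweepingSphere, which moves the actor along world X and yaws it, scaling MovementRate and RotationSpeed by delta time for frame-rate independence.
; It then uses debug draw calls to show a sphere at the actor's location and a forward-pointing line capped with a point, so the line sweeps as the actor rotates.
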(event `self.ReceiveTick`
  (params (DeltaSeconds :type "Float (single-precision)"))
  (`self.LineSweepingSphere` DeltaSeconds))

(fn `LineSweepingSphere`
  (params (DeltaTime :type "Float (single-precision)"))
  (locals (MovementRate :type "Float (double-precision)" :default 50.0) (RotationSpeed :type "Float (double-precision)" :default 45.0))
  (bind _returnvalue (`self.K2_GetActorLocation`))
  (`self.K2_AddActorWorldOffset` (`KismetMathLibrary.MakeVector` (* DeltaTime (`local.MovementRate`))))
  (`KismetSystemLibrary.DrawDebugSphere` (`self.K2_GetActorLocation`) 50.0 12 (struct :`R` 1.0 :`G` 1.0 :`B` 1.0 :`A` 1.0) 0.0 1.0)
  (`self.K2_AddActorWorldRotation` (`KismetMathLibrary.MakeRotator` 0.0 0.0 (* DeltaTime (`local.RotationSpeed`))))
  (`KismetSystemLibrary.DrawDebugLine` _returnvalue (+ _returnvalue (* (`self.GetActorForwardVector`) 150.0)) (struct :`R` 1.0 :`G` 1.0 :`B` 1.0 :`A` 1.0) 0.0 1.0)
  (`KismetSystemLibrary.DrawDebugPoint` (+ (`self.K2_GetActorLocation`) (* (`self.GetActorForwardVector`) 150.0)) 25.0 (struct :`R` 1.0 :`G` 1.0 :`B` 1.0 :`A` 1.0))
  (return))

(fn `UserConstructionScript`)